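; Event-activated gameplay ability that drives a distance-based cue effect on a target and destroys the player's pawn on touching it.
; It executes a GameplayCue with itself as SourceObject, allowing the cue actor to be registered through SetGameplayCue.
; The cue's overlaps toggle visibility and ability tick, which scales intensity up with distance from the target.
; Capsule overlap with the target unbinds, destroys the pawn and ends the ability.
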(event Custom|InRange_Event
  (params (OverlappedActor :type Actor%20Object%20Reference) (OtherActor :type Actor%20Object%20Reference))
  ;[0 0.001847 0.015] SetGameplayCue initializes the ability gameplaycue and bind events.
  ; Hide the GameplayCue and the target actor accordingly.
  (Utilities|Casting|CastToBP_XoneCharacter OtherActor)
  (Rendering|SetActorHiddenInGame (Components|GetOwner OverlappedActor) false)
  (Rendering|SetActorHiddenInGame (Variables|Default|GetGameplay%20Cue) false)
  (Development|PrintString "Player In Range")
  ;[0 0.001847 0.015] Provide control on the AbilityTick preventing unnecessary logic execution.
  (Class|XoneGameplayAbility|EnableAbilityTick))

(event Custom|OutOfRange_Event
  (params (OverlappedActor :type Actor%20Object%20Reference) (OtherActor :type Actor%20Object%20Reference))
  ;[0 0.001847 0.015] SetGameplayCue initializes the ability gameplaycue and bind events.
  ; Hide the GameplayCue and the target actor accordingly.
  (bind _asbp_xone_character (Utilities|Casting|CastToBP_XoneCharacter OtherActor))
  (if (Variables|/Game/Xone/BP_XoneCharacter.BP_XoneCharacter_C|GetIsDead _asbp_xone_character)
    _
    (else
      (Rendering|SetActorHiddenInGame (Components|GetOwner OverlappedActor) true)))
  (Rendering|SetActorHiddenInGame (Variables|Default|GetGameplay%20Cue) true)
  (Development|PrintString "Player Out Of Range")
  ;[0 0.001847 0.015] Provide control on the AbilityTick preventing unnecessary logic execution.
  (Class|XoneGameplayAbility|DisableAbilityTick))

(event Custom|OnCharacterOverlap_Event
  (params (OverlappedComponent :type Primitive%20Component%20Object%20Reference) (OtherActor :type Actor%20Object%20Reference) (OtherComp :type Primitive%20Component%20Object%20Reference) (OtherBodyIndex :type Integer) (bFromSweep :type Boolean) (SweepResult :type Hit%20Result%20Structure%20%28by%20ref%29))
  ;[0 0.015 0] If the player touches the object
  (if (== OtherActor (Variables|Default|GetTarget))
    ;[0.015 0.015 0.015] Cleaning
    (Collision|UnbindEventfromOnComponentBeginOverlap (Variables|/Script/Engine.Character|GetCapsuleComponent (Class|XoneGameplayAbility|GetXoneCharacterfromActorInfo)) (delegate Custom|OnCharacterOverlap_Event))
    (Class|XoneGameplayAbility|DisableAbilityTick)
    ;[0 0.015 0] Destroy player’s pawn and end ability
    (Actor|DestroyActor (Class|XoneGameplayAbility|GetXoneCharacterfromActorInfo))
    (Ability|EndAbility)))

(event EventOnAbilityTick
  (params (DeltaTime :type Float%20%28single-precision%29))
  (bind (_intensity _distance) (CallFunction|GetDistanceBasedIntensity))
  ;[0 0.015 0] AbilityTick
  (bind _gameplay_cue (Variables|Default|GetGameplay%20Cue)
    (:then
      (Default|SetIntensity _gameplay_cue _intensity)
      (Development|PrintText (Utilities|Text|FormatText "Intensity: {Effect} 
Distance: {Distance}" _intensity _distance) true false "(R=0.000000,G=0.660000,B=1.000000,A=1.000000)" DeltaTime))
    (:else)))

(event Ability|EventOnEndAbility
  (params (bWasCancelled :type Boolean))
  ;[0.015 0.015 0.015] OnEndAbility
  (Development|PrintString "Pawn Destroyed" true true "(R=0.484375,G=0.009623,B=0.000000,A=1.000000)" 5.0)
  ;;[0.015 0.015 0.015] Cleaning
  (Variables|Default|SetTarget 0)
  (Variables|Default|SetGameplay%20Cue 0))

(event Ability|EventActivateAbilityFromEvent
  (params (EventData :type Gameplay%20Event%20Data%20Structure%20%28by%20ref%29))
  ;[0.015 0.015 0.015] ActivateAbilityFromEvent
  ;;[0.015 0.015 0.015] Bind event to player's capsule component
  (Collision|AssignOnComponentBeginOverlap (Variables|/Script/Engine.Character|GetCapsuleComponent (Class|XoneGameplayAbility|GetXoneCharacterfromActorInfo)) (EventDispatchers|CreateEvent :!event Custom|OnCharacterOverlap_Event))
  ;;[0 0.015 0] Execute GameplaCue. Passing Self allows the GameplayCue to provide its reference.
  (bind _output_get (Variables|Default|SetTarget (Utilities|Struct|BreakGameplayEventData EventData)))
  (GameplayCue|ExecuteGameplayCueOnActor(Burst) _output_get "(TagName=\"GameplayCue.Test\")" (Ability|GameplayCue|MakeGameplayCueParameters :SourceObject self))
  (Class|XoneGameplayAbility|EnableAbilityTick))

(fn SetGameplayCue
  (params (GameplayCue :type GNC%20Gamplay%20Cue%20Object%20Reference))
  (bind _output_get (Variables|Default|SetGameplay%20Cue GameplayCue))
  (Collision|BindEventtoOnActorBeginOverlap _output_get (EventDispatchers|CreateEvent :!event Custom|InRange_Event))
  (Collision|BindEventtoOnActorEndOverlap _output_get (EventDispatchers|CreateEvent :!event Custom|OutOfRange_Event)))

(fn GetDistanceBasedIntensity
  (bind _target (Variables|Default|GetTarget)
    (:then
      (return (Math|Float|MapRangeClamped (Math|Vector|Distance(Vector) (Transformation|GetActorLocation _target) (Transformation|GetActorLocation (Ability|GetAvatarActorfromActorInfo))) 3e+02 1e+03 1.0 2e+02) (Math|Vector|Distance(Vector) (Transformation|GetActorLocation _target) (Transformation|GetActorLocation (Ability|GetAvatarActorfromActorInfo)))))
    (:else)))